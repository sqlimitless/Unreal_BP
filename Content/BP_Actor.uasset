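; Actor that moves along world +X until it overlaps another actor, then reports its arrival.
; While MoveAble is true, Tick offsets its location by a new random speed each frame scaled by DeltaSeconds, without sweeping.
; ActorBeginOverlap broadcasts OnArrive with the actor's Name variable and clears MoveAble to stop movement.
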(event `self.ReceiveActorBeginOverlap`
  (params (OtherActor :type "Actor Object Reference"))
  (`self.OnArrive` (`self.name`))
  (set `self.moveAble` false))

(event `self.ReceiveTick`
  (params (DeltaSeconds :type "Float (single-precision)"))
  (if (`self.moveAble`)
    (`self.K2_SetActorLocation` (+ (`self.K2_GetActorLocation`) (`KismetMathLibrary.MakeVector` (* DeltaSeconds (`KismetMathLibrary.RandomIntegerInRange` 1 5000)))))))

(fn `UserConstructionScript`)